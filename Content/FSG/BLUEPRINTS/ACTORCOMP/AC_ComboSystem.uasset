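; Actor component for a combo attack system that tracks the current combo and attack count, apparently work in progress.
; IniciarCombo, at attack index zero, looks up a montage for the current combo in ListaCombos, then increments the counter and broadcasts it, or resets if none is valid.
; GetMontage ignores input key and index, returning the first sequence entry.
; AtaqueConfirmado and AtaqueActivo are empty stubs.
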(event EventBeginPlay)

(event EventTick
  (params (DeltaSeconds :type Float%20%28single-precision%29)))

(fn GetMontage
  (params (ComboName :type Enum_Combos%20Enum :default "NewEnumerator0") (InputKey :type Enum_InputKey%20Enum :default "NewEnumerator0") (Index :type Integer))
  (LocalVariables|SetL_Montage 0)
  (bind _array_element (Utilities|Array|ForEachLoopwithBreak (Variables|Combos|GetListaCombos) :!label _label)
    (:LoopBody
      (if (Utilities|Enum|Equal(Enum) (.Nombre (Utilities|Struct|BreakF_Combos _array_element)) ComboName)
        (bind (_array_element_2 _array_index) (Utilities|Array|ForEachLoopwithBreak (.Secuencia (Utilities|Struct|BreakF_Combos _array_element)))
          (:LoopBody
            (if true
              (LocalVariables|SetL_Montage (.Montage (Utilities|Struct|BreakF_InfoCombo _array_element_2)))
              (goto _label Break)
              (else
                (return 0)))))
        (else
          (return 0))))
    (:Completed
      (return (LocalVariables|GetL_Montage)))))

(fn AtaqueConfirmado)

(fn AtaqueActivo)

(fn ComboReset
  (Variables|Default|SetComboActivado false)
  (Variables|Default|SetContadorAtaques 0)
  (Variables|Default|SetComboActual "NewEnumerator0")
  (Default|CallComboReiniciado))

(fn SetCombo
  (params (Combo :type Enum_Combos%20Enum :default "NewEnumerator0"))
  (Variables|Default|SetComboActual Combo))

(fn IniciarCombo
  (params (Combo :type Enum_Combos%20Enum :default "NewEnumerator0") (InputKey :type Enum_InputKey%20Enum :default "NewEnumerator0") (AtaqueIndex :type Integer))
  (if (== AtaqueIndex 0)
    (bind _combomontage (CallFunction|GetMontage (Variables|Default|GetComboActual) InputKey (Variables|Default|GetContadorAtaques)))
    (Utilities|IsValid _combomontage
      (:Is%20Valid
        (Math|Integer|IncrementInt (Variables|Default|GetContadorAtaques)
          (:%20%20
            (Default|CallPlayAnimMontage _combomontage 0.0))))
      (:Is%20Not%20Valid
        (CallFunction|ComboReset)))))