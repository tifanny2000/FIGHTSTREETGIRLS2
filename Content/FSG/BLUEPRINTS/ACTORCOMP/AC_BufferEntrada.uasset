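; AC_BufferEntrada is an actor component that implements an input buffer, holding one enum key until it is consumed.
; ActualizarKey overwrites the stored key and consumes it immediately when the buffer is closed; while open, it keeps only the latest key.
; Closing the buffer consumes the stored key, which broadcasts it and resets it to the first enum value.
; Dispatchers announce opening, closing and consumption, so other logic reacts without polling.
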(event EventBeginPlay)

(event EventTick
  (params (DeltaSeconds :type Float%20%28single-precision%29)))

(fn ActualizarKey
  (params (NuevoKey :type Enum_BufferEntrada%20Enum :default "NewEnumerator0"))
  (Variables|Default|SetKeyAlmacenado NuevoKey)
  (if (not (Variables|Default|GetEstaAbierto))
    (CallFunction|ConsumirBuffer)))

(fn ConsumirBuffer
  (Default|CallONBufferConsumido (Variables|Default|GetKeyAlmacenado))
  (Variables|Default|SetKeyAlmacenado "NewEnumerator0"))

(fn CerrarBuffer
  (Variables|Default|SetEstaAbierto false)
  (Default|CallONBufferCerrado)
  (CallFunction|ConsumirBuffer))

(fn AbrirBuffer
  (Variables|Default|SetEstaAbierto true)
  (Default|CallONBufferAbierto))

(fn GetKeyAlmacenado
  (return (Variables|Default|GetKeyAlmacenado)))