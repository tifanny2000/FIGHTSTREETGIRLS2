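; Hitbox actor that shows a hit volume and deals damage to Dummy actors overlapping it.
; SpawnHitbox sets the display material by hitbox type (strike or damage area), moves the display to HitboxLocation, reveals it, then runs CheckCollision.
; CheckCollision polls overlapping actors once per call, excluding the owner, and passes HitboxDamage and ReactionIndex to each Dummy's TomarDaño.
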(event Custom|SpawnHitbox
  (switch Utilities|FlowControl|Switch|SwitchonEnum_HitboxType (Variables|Default|GetHitboxType)
    (:NewEnumerator0
      (Rendering|Material|SetMaterial (Variables|Default|GetHitboxDisplay) 0 0))
    (:NewEnumerator1
      (Rendering|Material|SetMaterial (Variables|Default|GetHitboxDisplay) 0 0)))
  (Transformation|SetWorldLocation (Variables|Default|GetHitboxDisplay) (Variables|Default|GetHitboxLocation) false false)
  (Rendering|SetVisibility (Variables|Default|GetHitboxDisplay) true false)
  (CallFunction|CheckCollision))

(event Custom|CheckCollision
  (for _array_element (Collision|GetOverlappingActors 0 :!class /Script/Engine.Actor)
    (if (!= _array_element (Components|GetOwner))
      (bind _asdummy (Utilities|Casting|CastToDummy _array_element))
      (Default|TomarDaño _asdummy (Variables|Default|GetReactionIndex) (Variables|Default|GetHitboxDamage)))))

(fn ConstructionScript)