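; Behavior tree service that picks the Dummy enemy's behavior state from its distance to the FightGirl player.
; On search start it caches the Dummy pawn and player character.
; Each tick it compares their distance to SafeDistance and DistanciadeAtaque (attack range), writing one of three enum states to the BehaviorKey blackboard entry.
; It reads the TargetKey detection flag, but the following branch is hardwired true, so detection does not gate the choice.
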(event EventReceiveSearchStartAI
  (params (OwnerController :type AI%20Controller%20Object%20Reference) (ControlledPawn :type Pawn%20Object%20Reference))
  (bind _asdummy (Utilities|Casting|CastToDummy ControlledPawn))
  (Variables|Default|SetDummyRef _asdummy)
  (bind _asfight_girl_bp (Utilities|Casting|CastToFightGIrlBP (Game|GetPlayerCharacter 0)))
  (Variables|Default|SetFightGirlRef _asfight_girl_bp))

(event EventTick
  (params (OwnerActor :type Actor%20Object%20Reference) (DeltaSeconds :type Float%20%28single-precision%29))
  (Variables|Default|GetDummyRef
    (:then
      (Variables|Default|SetDetected (Class|BTFunctionLibrary|GetBlackboardValueasBool (Variables|Default|GetTargetKey)))
      (if true
        (if (>= (Math|Vector|Distance(Vector) (Transformation|GetActorLocation (Variables|Default|GetDummyRef)) (Transformation|GetActorLocation (Variables|Default|GetFightGirlRef))) (Variables|Default|GetSafeDistance))
          (Utilities|SetBehavior "NewEnumerator0")
          (elif (>= (Math|Vector|Distance(Vector) (Transformation|GetActorLocation (Variables|Default|GetDummyRef)) (Transformation|GetActorLocation (Variables|Default|GetFightGirlRef))) (Variables|Default|GetDistanciadeAtaque))
            (Utilities|SetBehavior "NewEnumerator1")
            (else
              (Utilities|SetBehavior "NewEnumerator3"))))))
    (:else)))