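; Dummy is a character in the AI folder that turns to face another actor and reacts to the fighter FightGIrlBP.
; Each tick it compares Y positions with OtherActor and mirrors its mesh by flipping the Y scale, tracking the state in EstaGirado.
; When FightGIrlBP overlaps its Box with ReactionTrigger set, it plays the montage that ReactionInt selects from ReactionMontages, and any such overlap prints a debug string.
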(event OnComponentBeginOverlap(Box)
  (params (OverlappedComponent :type Primitive%20Component%20Object%20Reference) (OtherActor :type Actor%20Object%20Reference) (OtherComp :type Primitive%20Component%20Object%20Reference) (OtherBodyIndex :type Integer) (bFromSweep :type Boolean) (SweepResult :type Hit%20Result%20Structure%20%28by%20ref%29))
  (bind _asfight_girl_bp (Utilities|Casting|CastToFightGIrlBP OtherActor))
  (Development|PrintString "Hello")
  (if (Variables|/Game/FSG/BLUEPRINTS/FightGIrlBP.FightGIrlBP_C|GetReactionTrigger _asfight_girl_bp)
    (Animation|PlayAnimMontage (Utilities|Array|Get(acopy) (Variables|Default|GetReactionMontages) (Variables|/Game/FSG/BLUEPRINTS/FightGIrlBP.FightGIrlBP_C|GetReactionInt _asfight_girl_bp)) 1.0 "None")))

(event EventBeginPlay)

(event EventTick
  (params (DeltaSeconds :type Float%20%28single-precision%29))
  (bind _mesh (Variables|Character|GetMesh))
  (bind _mesh_2 (Variables|Character|GetMesh))
  (bind _relativescale3d (Variables|/Script/Engine.SceneComponent|GetRelativeScale3D _mesh))
  (bind _relativescale3d_2 (Variables|/Script/Engine.SceneComponent|GetRelativeScale3D _mesh_2))
  (Utilities|IsValid (Variables|Default|GetOtherActor)
    (:Is%20Valid
      (if (>= (.y (Transformation|GetActorLocation (Variables|Default|GetOtherActor))) (.y (Transformation|GetActorLocation)))
        (if (Variables|Default|GetEstaGirado)
          (Transformation|SetRelativeScale3D (Variables|Character|GetMesh) (Math|Vector|MakeVector (.x _relativescale3d_2) (Math|Float|Absolute(Float) (.y _relativescale3d_2)) (.z _relativescale3d_2)))
          (Variables|Default|SetEstaGirado false))
        (elif (not (Variables|Default|GetEstaGirado))
          (Transformation|SetRelativeScale3D (Variables|Character|GetMesh) (Math|Vector|MakeVector (.x _relativescale3d) (* (.y _relativescale3d) -1.0) (.z _relativescale3d)))
          (Variables|Default|SetEstaGirado true))))))

(fn ConstructionScript)